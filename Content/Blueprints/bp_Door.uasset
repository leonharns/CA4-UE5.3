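; Interactable door that opens only once the game mode's CollLeft counter reaches zero.
; Overlap of its Box by the third-person character enables input on the door, and leaving disables it.
; Pressing E either plays a timeline that lerps the Cube upward or, while the count is nonzero, shows a not-all-collected widget.
; A separate OpenDoor event plays the same timeline without the check.
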(event `Key|E`
  (params (Key :type "Key Structure"))
  (:`Pressed`
    (bind _asbp_third_person_game_mode (cast `/Game/ThirdPerson/Blueprints/BP_ThirdPersonGameMode` (`GameplayStatics.GetGameMode`)))
    (if (== (`/Game/ThirdPerson/Blueprints/BP_ThirdPersonGameMode.CollLeft` _asbp_third_person_game_mode) 0)
      (bind (_direction _opn_track) (`Timeline|Open Door T` :!label _label)
        (:`Update`
          (`SceneComponent.K2_SetRelativeLocation` (`self.Cube`) (`KismetMathLibrary.VLerp` (0.0 0.0 0.0) (0.0 0.0 300.0) _opn_track) false false)))
      (else
        (bind _returnvalue (`|CreateWidget` "/Game/Blueprints/bp_notallcollect.bp_notallcollect_C"))
        (`UserWidget.AddToViewport` _returnvalue 0)))))

(event `Open Door`
  (goto _label))

(event `self.Box.OnComponentBeginOverlap`
  (params (OverlappedComponent :type "PrimitiveComponent Object Reference") (OtherActor :type "Actor Object Reference") (OtherComp :type "PrimitiveComponent Object Reference") (OtherBodyIndex :type Integer) (bFromSweep :type Boolean) (SweepResult :type "HitResult Structure (by ref)"))
  (cast `/Game/ThirdPerson/Blueprints/BP_ThirdPersonCharacter` OtherActor)
  (`self.EnableInput` (`GameplayStatics.GetPlayerController` 0)))

(event `self.Box.OnComponentEndOverlap`
  (params (OverlappedComponent :type "PrimitiveComponent Object Reference") (OtherActor :type "Actor Object Reference") (OtherComp :type "PrimitiveComponent Object Reference") (OtherBodyIndex :type Integer))
  (cast `/Game/ThirdPerson/Blueprints/BP_ThirdPersonCharacter` OtherActor)
  (`self.DisableInput` (`GameplayStatics.GetPlayerController` 0)))

(fn `UserConstructionScript`)