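; Cannon actor that launches Ball actors at random intervals, starting with one shot on BeginPlay.
; Tick runs into a 1–3 second random Delay before each FireCannon, so the latent node throttles the repeat rate; its Active check has empty branches.
; FireCannon plays a quiet explosion sound at the mesh and spawns a Ball at the Sphere's location plus CannonOffset, rotated to the Scene component's orientation.
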(event `self.ReceiveBeginPlay`
  (`self.FireCannon`))

(event `self.ReceiveTick`
  (params (DeltaSeconds :type "Float (single-precision)"))
  (if (`self.Active`)
    _
    (else
      _))
  (`KismetSystemLibrary.Delay` (`KismetMathLibrary.RandomFloatInRange` 1.0 3.0))
  (`self.FireCannon`))

(event `FireCannon`
  (bind _returnvalue (`SceneComponent.K2_GetComponentRotation` (`self.Scene`)))
  (`GameplayStatics.PlaySoundAtLocation` "/Game/StarterContent/Audio/Explosion01.Explosion01" (`SceneComponent.K2_GetComponentLocation` (`self.StaticMesh`)) (struct) 0.1 1.0 0.0 null null null null)
  (`|SpawnActorFromClass` "/Game/Blueprints/Ball.Ball_C" (`KismetMathLibrary.MakeTransform` (+ (`SceneComponent.K2_GetComponentLocation` (`self.Sphere`)) (`KismetMathLibrary.GreaterGreater_VectorRotator` (`self.cannon offset`) _returnvalue)) _returnvalue) "Undefined" "MultiplyWithRoot" null null))

(fn `UserConstructionScript`)