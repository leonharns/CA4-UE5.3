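; Checkpoint Blueprint that shows its active state with a fire effect.
; Activate spawns the P_Fire emitter at the ParticleSystem component's transform, only if no valid Fire exists, then plays Fire01 for half a second before stopping it.
; Deactivate destroys the stored Fire component, allowing a later activation to spawn it again.
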(event `Activate`
  (bind _fire01 (`self.Fire01`))
  (bind (_returnvalue_location _returnvalue_rotation _returnvalue_scale) (`KismetMathLibrary.BreakTransform` (`SceneComponent.K2_GetComponentToWorld` (`self.ParticleSystem`))))
  (`/Engine/EditorBlueprintResources/StandardMacros.IsValid` (`self.fire`)
    (:`Is Not Valid`
      (bind _returnvalue (`GameplayStatics.SpawnEmitterAtLocation` "/Game/StarterContent/Particles/P_Fire.P_Fire" _returnvalue_location _returnvalue_rotation _returnvalue_scale))
      (set `self.fire` _returnvalue)
      (`AudioComponent.Play` _fire01 0.0)
      (`KismetSystemLibrary.Delay` 0.5)
      (`AudioComponent.Stop` _fire01))))

(event `Deactivate`
  (bind _fire (`self.fire`))
  (`/Engine/EditorBlueprintResources/StandardMacros.IsValid` _fire
    (:`Is Valid`
      (`ActorComponent.K2_DestroyComponent` _fire))))

(fn `UserConstructionScript`)